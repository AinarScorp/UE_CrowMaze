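; BP_SaveGame is a save-game Blueprint that holds the HighScoreValues array of high scores.
; AddHighScoreValue adds the first score directly to an empty array, and otherwise inserts the new score at the index returned by FindInsertIndex, keeping the list ordered without re-sorting.
; The list is not trimmed, and the EventGraph contains only disconnected nodes that never run.
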(fn AddHighScoreValue
  (params (HighScoreToAdd :type Integer))
  (bind _highscorevalues (Variables|Default|GetHighScoreValues))
  (LocalVariables|SetToAdd HighScoreToAdd)
  (if (Utilities|Array|IsEmpty (Variables|Default|GetHighScoreValues))
    (Utilities|Array|Add (Variables|Default|GetHighScoreValues) (LocalVariables|GetToAdd))
    (else
      (Utilities|Array|Insert _highscorevalues (LocalVariables|GetToAdd) (Class|SortingArray|FindInsertIndex _highscorevalues (LocalVariables|GetToAdd))))))