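; Moving barrier tile for the crow endless runner, exposing its half size and a 3x3 grid of obstacle points.
; Each tick it steps along MoveDirection via constant interpolation, using the GameMoveSpeed read once from BP_CrowGameMode at BeginPlay as target offset.
; When a sphere component of the tagged crow player overlaps EndPoint, it asks the game mode to spawn another tile and sets a short lifespan on itself.
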(event OnComponentBeginOverlap(EndPoint)
  (params (OverlappedComponent :type Primitive%20Component%20Object%20Reference) (OtherActor :type Actor%20Object%20Reference) (OtherComp :type Primitive%20Component%20Object%20Reference) (OtherBodyIndex :type Integer) (bFromSweep :type Boolean) (SweepResult :type Hit%20Result%20Structure%20%28by%20ref%29))
  (if (== OtherActor (Variables|Default|GetCrowPlayer))
    (Utilities|Casting|CastToSphereComponent OtherComp)
    (bind _asbp_crow_game_mode (Utilities|Casting|CastToBP_CrowGameMode (Game|GetGameMode)))
    (Default|SpawnTile _asbp_crow_game_mode false)
    (Actor|SetLifeSpan 3.0)))

(event EventBeginPlay
  (CallFunction|SetHalfSize)
  (CallFunction|SetMoveSpeed)
  (CallFunction|FindCrowPlayer))

(event Collision|EventActorBeginOverlap
  (params (OtherActor :type Actor%20Object%20Reference)))

(event EventTick
  (params (DeltaSeconds :type Float%20%28single-precision%29))
  (bind _returnvalue (Transformation|GetActorLocation))
  (Transformation|SetActorLocation (Math|Interpolation|VInterptoConstant _returnvalue (+ _returnvalue (* (Variables|Default|GetMoveDirection) (Variables|Default|GetMoveSpeed))) DeltaSeconds 2e+03) false false))

(fn ConstructionScript)

(fn GetHalfSize
  (return (Variables|Default|GetHalfSize)))

(fn SetMoveSpeed
  (bind _asbp_crow_game_mode (Utilities|Casting|CastToBP_CrowGameMode (Game|GetGameMode)))
  (Variables|Default|SetMoveSpeed (Variables|/Game/Blueprints/BP_CrowGameMode.BP_CrowGameMode_C|GetGameMoveSpeed _asbp_crow_game_mode)))

(fn SetHalfSize
  (Variables|Default|SetHalfSize (* (.x (Transformation|GetWorldScale (Variables|Default|GetBarriers))) 1e+02)))

(fn FindCrowPlayer
  (bind _outactors (Actor|GetAllActorswithTag "CrowPlayer"))
  (if (> (Utilities|Array|Length _outactors) 0)
    (bind _asbp_crow (Utilities|Casting|CastToBP_Crow (Utilities|Array|Get(acopy) _outactors)))
    (Variables|Default|SetCrowPlayer _asbp_crow)))

(fn GetObstaclePoints
  (return (Utilities|Array|MakeArray (Variables|Default|GetBP_ObstaclePointTopLeft) (Variables|Default|GetBP_ObstaclePointTopMiddle) (Variables|Default|GetBP_ObstaclePointTopRight) (Variables|Default|GetBP_ObstaclePointCenterLeft) (Variables|Default|GetBP_ObstaclePointCenterMiddle) (Variables|Default|GetBP_ObstaclePointCenterRight) (Variables|Default|GetBP_ObstaclePointBottomLeft) (Variables|Default|GetBP_ObstaclePointBottomMiddle) (Variables|Default|GetBP_ObstaclePointBottomRight))))