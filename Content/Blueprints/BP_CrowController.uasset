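; BP_CrowController is a controller, apparently for a crow, that levels the control rotation's roll when no buttons are pressed.
; Each Tick, while PressingButtons is false and roll is non-zero, it moves roll toward zero at a constant rate, preserving pitch and yaw.
; Roll above 180 degrees is wrapped to a negative angle first, so it levels along the shortest path.
; Nothing in this graph sets PressingButtons.
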(event EventBeginPlay)

(event EventTick
  (params (DeltaSeconds :type Float%20%28single-precision%29))
  (bind _returnvalue (Pawn|GetControlRotation :!class /Script/Engine.Controller))
  (bind (_roll _pitch _yaw) (Math|Rotator|BreakRotator _returnvalue))
  (if (and (not (Variables|Default|GetPressingButtons)) (!= _roll 0.0))
    (Pawn|SetControlRotation (Math|Rotator|MakeRotator (Math|Interpolation|FInterptoConstant (Math|Float|SelectFloat (- _roll 3.6e+02) _roll (> _roll 1.8e+02)) 0.0 DeltaSeconds 1e+02) _pitch _yaw))))

(fn ConstructionScript)