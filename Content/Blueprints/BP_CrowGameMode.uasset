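; BP_CrowGameMode is a game mode that builds endless terrain along the X axis from the player's starting position.
; BeginPlay measures a pooled tile's half size, lays a run of obstacle-free starting tiles, then pulls the spawn point back slightly.
; SpawnTile places BP_EndlessBariers actors from TerrainPool and, for non-starting tiles, spawns a random obstacle shape that builds itself on that tile.
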(event EventBeginPlay
  (bind _output_get (Variables|Default|SetPlayerStartPos (Transformation|GetActorLocation (Game|Player|GetPlayerPawn 0))))
  (Variables|Default|SetSpawnPos _output_get)
  (CallFunction|SpawnStartingTiles (Variables|Default|GetNumberOfStartingTiles)))

(event EventTick
  (params (DeltaSeconds :type Float%20%28single-precision%29)))

(fn ConstructionScript)

(fn SpawnTile
  (params (StartingTile :type Boolean))
  (bind _terrainpool (Variables|Default|GetTerrainPool)
    (:then
      (bind _returnvalue (Class|ActorPool|GetPooledActorBP _terrainpool))
      (Class|PoolableActorAbstact|SpawnActor _returnvalue (Variables|Default|GetSpawnPos) (Transformation|GetActorRotation _returnvalue))
      (if StartingTile
        _
        (else
          (bind _asbp_endless_bariers (Utilities|Casting|CastToBP_EndlessBariers _returnvalue))
          (bind _returnvalue_2 (Game|SpawnActorfromClass (.OutItem (Utilities|Array|Random (Variables|Default|GetObstacleShapes))) (Math|Transform|MakeTransform "0, 0, 0" "0, 0, 0" "1.000000,1.000000,1.000000") "Undefined" _asbp_endless_bariers 0))
          (Class|Obstacle|CreateObstacle _returnvalue_2 _asbp_endless_bariers)))
      (return))
    (:else)))

(fn SpawnStartingTiles
  (params (NumberOfTiles :type Integer))
  (CallFunction|SetHalfSize)
  (for _index (range 0 NumberOfTiles)
    (CallFunction|SpawnTile true)
    (CallFunction|MoveSpawnPosFurther))
  (Variables|Default|SetSpawnPos (Math|Vector|MakeVector (- (.x (Variables|Default|GetSpawnPos)) (/ (Variables|Default|GetHalfSize) 2.0)) (.y (Variables|Default|GetSpawnPos)) (.z (Variables|Default|GetSpawnPos)))))

(fn SetHalfSize
  (bind _returnvalue (Class|ActorPool|GetPooledActorBP (Variables|Default|GetTerrainPool)))
  (Utilities|IsValid _returnvalue
    (:Is%20Valid
      (bind _asbp_endless_bariers (Utilities|Casting|CastToBP_EndlessBariers _returnvalue))
      (Variables|Default|SetHalfSize (Default|GetHalfSize _asbp_endless_bariers)))))

(fn MoveSpawnPosFurther
  (Variables|Default|SetSpawnPos (Math|Vector|MakeVector (+ (Variables|Default|GetHalfSize) (.x (Variables|Default|GetSpawnPos))) (.y (Variables|Default|GetSpawnPos)) (.z (Variables|Default|GetSpawnPos)))))