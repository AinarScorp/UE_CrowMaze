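; Game mode for an endless runner that builds terrain ahead of the player and tracks score and game speed.
; On BeginPlay, it lays starting tiles from TerrainPool along X, spaced by the tile's HalfSize.
; Non-starting SpawnTile calls raise the score and give tiles a 50% chance of a random obstacle shape.
; Event dispatcher calls and the speed-up every ten points are disconnected, so they never run.
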(event EventBeginPlay
  (Variables|Default|SetSpawnPos (Transformation|GetActorLocation (Game|Player|GetPlayerPawn 0)))
  (CallFunction|SpawnStartingTiles (Variables|Default|GetNumberOfStartingTiles)))

(fn ConstructionScript)

(fn SpawnTile
  (params (StartingTile :type Boolean))
  (bind _terrainpool (Variables|Default|GetTerrainPool)
    (:then
      (bind _returnvalue (Class|ActorPool|GetPooledActorBP _terrainpool))
      (Class|PoolableActorAbstact|SpawnActor _returnvalue (Variables|Default|GetSpawnPos) (Transformation|GetActorRotation _returnvalue))
      (if StartingTile
        _
        (else
          (CallFunction|IncreaseScore)
          (if (Math|Random|RandomBoolwithWeight 0.5)
            (bind _asbp_endless_bariers (Utilities|Casting|CastToBP_EndlessBariers _returnvalue))
            (bind _returnvalue_2 (Game|SpawnActorfromClass (.OutItem (Utilities|Array|Random (Variables|Default|GetObstacleShapes))) (Math|Transform|MakeTransform "0, 0, 0" "0, 0, 0" "1.000000,1.000000,1.000000") "AlwaysSpawn" _asbp_endless_bariers 0))
            (Class|Obstacle|CreateObstacle _returnvalue_2 _asbp_endless_bariers))))
      (return))
    (:else)))

(fn SpawnStartingTiles
  (params (NumberOfTiles :type Integer))
  (CallFunction|SetHalfSize)
  (for _index (range 0 NumberOfTiles)
    (CallFunction|SpawnTile true)
    (CallFunction|MoveSpawnPosFurther))
  (Variables|Default|SetSpawnPos (Math|Vector|MakeVector (- (.x (Variables|Default|GetSpawnPos)) (/ (Variables|Default|GetHalfSize) 2.0)) (.y (Variables|Default|GetSpawnPos)) (.z (Variables|Default|GetSpawnPos))))
  (Variables|Default|SetGameIsOn true)
  (CallFunction|ChangeGameSpeed (Variables|Default|GetGameMoveSpeed)))

(fn SetHalfSize
  (bind _returnvalue (Class|ActorPool|GetPooledActorBP (Variables|Default|GetTerrainPool)))
  (Utilities|IsValid _returnvalue
    (:Is%20Valid
      (bind _asbp_endless_bariers (Utilities|Casting|CastToBP_EndlessBariers _returnvalue))
      (Variables|Default|SetHalfSize (Default|GetHalfSize _asbp_endless_bariers)))))

(fn MoveSpawnPosFurther
  (Variables|Default|SetSpawnPos (Math|Vector|MakeVector (+ (Variables|Default|GetHalfSize) (.x (Variables|Default|GetSpawnPos))) (.y (Variables|Default|GetSpawnPos)) (.z (Variables|Default|GetSpawnPos)))))

(fn IncreaseScore
  (bind _result (Math|Float|IncrementFloat (Variables|Default|GetCurrentScore))))

(fn IncreaseSpeed
  (CallFunction|ChangeGameSpeed (+ (Variables|Default|GetSpeedIncrease) (Variables|Default|GetGameMoveSpeed))))

(fn ChangeGameSpeed
  (params (NewSpeed :type Float%20%28double-precision%29))
  (bind _output_get (Variables|Default|SetGameMoveSpeed NewSpeed)))